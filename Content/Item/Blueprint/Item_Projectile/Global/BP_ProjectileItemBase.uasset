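; Base Blueprint for projectile item pickups that give ammo to a weapon the player already has.
; On pickup, a helper validates that the causer is a Player-tagged MainCharacterBase and fetches its weapon inventory.
; If the inventory contains the weapon matching ItemID, a DoOnce-guarded call tries to add AmmoCount.
; Success spawns an end effect, plays a 2D sound and destroys the item, while failure resets the guard.
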(event EventOnItemPicked
  (params (Causer :type Actor%20Object%20Reference))
  (bind _itemid (Variables|Default|GetItemID))
  (bind _returnvalue (Math|Conversions|ToInteger(Byte) _itemid))
  ;[1 0.2846 0.4761 1 35] BP_ImplementableEvent
  (bind _returnvalue_2 (|ValidityCheck&GetWeaponInventoryRef Causer Causer Causer)
    (:Is%20Valid
      (bind _returnvalue_3 (Class|WeaponInventoryBase|GetWeaponIsContained _returnvalue_2 _returnvalue))
      (if _returnvalue_3
        (Utilities|FlowControl|DoOnce false :!label _label
          (:Completed
            (bind _returnvalue_4 (Class|WeaponInventoryBase|TryAddAmmotoWeapon _returnvalue_2 _returnvalue (Variables|Gameplay|Settings|GetAmmoCount)))
            (if _returnvalue_4
              (Niagara|SpawnSystematLocation (Variables|Default|GetEndEffect) (Transformation|GetActorLocation) "0.000000,90.000000, 0")
              (Audio|PlaySound2D (Variables|Default|GetPickSound) 1.0 1.0 0.0 0 0)
              (Actor|DestroyActor)
              (else
                (goto _label Reset)))))))))

(fn ConstructionScript
  (|CallParentFunction))