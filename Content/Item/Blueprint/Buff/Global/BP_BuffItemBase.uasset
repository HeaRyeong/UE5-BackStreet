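; Base Blueprint for buff pickup items that grant a buff or debuff to the player character.
; When picked by a Player-tagged actor, it calls AddNewBuffDebuff on BP_MainCharacter with its type, duration and value, passing the game mode as causer.
; A DoOnce gate blocks repeat triggers; the item destroys itself on success and resets the gate if the buff is rejected.
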(event EventOnItemPicked
  (params (Causer :type Actor%20Object%20Reference))
  ;[0.7703 1 0.7232 1 36] BP_ImplementableEvent
  (Utilities|IsValid Causer
    (:Is%20Valid
      (if (Actor|ActorHasTag Causer "Player")
        (bind _asbp_main_character (Utilities|Casting|CastToBP_MainCharacter Causer))
        (Utilities|FlowControl|DoOnce false :!label _label
          (:Completed
            (bind _returnvalue (Class|MainCharacterBase|AddNewBuffDebuff _asbp_main_character false (Variables|Default|GetItemType) (Game|GetGameMode) (Variables|Gameplay|Buff|GetTotal%20Time) (Variables|Gameplay|Buff|GetValue)))
            (if _returnvalue
              (Actor|DestroyActor)
              (else
                (goto _label Reset)))))))))

(fn ConstructionScript)