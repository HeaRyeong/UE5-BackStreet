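; Base Blueprint for mission items that handles their pickup by the player.
; On pickup by a Player-tagged actor, it asks the level script's chapter manager to remove it from the mission items.
; Success spawns an enlarged end effect below the item and destroys it.
; A DoOnce blocks repeat pickups and resets with a debug print if removal fails.
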(event EventOnItemPicked
  (params (Causer :type Actor%20Object%20Reference))
  (bind _returnvalue (Class|ItemBase|GetLevelScriptRef))
  (bind _returnvalue_2 (Transformation|GetActorLocation))
  (bind _returnvalue_3 (Class|LevelScriptinGame|GetChapterManager _returnvalue))
  (bind (_x _y _z) (Math|Vector|BreakVector _returnvalue_2))
  ;[1 0.3666 0.9334 1 36] BP_ImplementableEvent
  (Utilities|IsValid Causer
    (:Is%20Valid
      (if (Actor|ActorHasTag Causer "Player")
        (Utilities|IsValid _returnvalue
          (:Is%20Valid
            (Utilities|IsValid _returnvalue_3
              (:Is%20Valid
                (Utilities|FlowControl|DoOnce false :!label _label
                  (:Completed
                    (bind _returnvalue_4 (Class|ChapterManagerBase|TryRemoveMissionItem _returnvalue_3 self))
                    (if _returnvalue_4
                      (Niagara|SpawnSystematLocation (Variables|Default|GetEndEffect) (Math|Vector|MakeVector _x _y (- _z 4.3e+02)) "0, 0, 0" "3.000000,3.000000,3.000000")
                      (Actor|DestroyActor)
                      (else
                        (Development|PrintString "Remove Mission Item : Failed" false)
                        (goto _label Reset)))))))))))))

(fn ConstructionScript)