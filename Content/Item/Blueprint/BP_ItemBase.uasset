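; BP_ItemBase is an item Blueprint, apparently a base class, that handles the item's activation sequence through the ActivateItem event.
; A Sequence starts two delayed branches: one turns on physics simulation for the root collision volume.
; The other, slightly later, plays a timeline that drives actor scale and uses a DoOnce on its update to activate the particle component once.
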(event EventActivateItem
  ;[1 0.6249 0.4631 1 36] BP_Implementable
  (Utilities|FlowControl|Sequence
    (:then_0
      (Utilities|FlowControl|Delay 0.25)
      (Physics|SetSimulatePhysics (Variables|Default|GetRootCollisionVolume) true))
    (:then_1
      (Utilities|FlowControl|Delay 0.5)
      (bind _scale (Timeline|타임라인_0 Play)
        (:Update
          (Transformation|SetActorScale3D (Math|Conversions|ToVector(Float) _scale))
          (Utilities|FlowControl|DoOnce false
            (:Completed
              (Components|Activation|Activate (Variables|Default|GetParticleComponent) false))))))))

(fn ConstructionScript)