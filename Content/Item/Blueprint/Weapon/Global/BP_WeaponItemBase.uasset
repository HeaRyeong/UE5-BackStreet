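; Base Blueprint for weapon items in the world that the player character can pick up.
; On the OnItemPicked event, it accepts only a valid causer tagged Player that casts to MainCharacterBase, then passes its ItemID as an integer to that character's PickWeapon.
; A DoOnce guards against repeat pickups: the item destroys itself on success and resets the gate when PickWeapon fails.
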(event EventOnItemPicked
  (params (Causer :type Actor%20Object%20Reference))
  ;[1 0.9696 0.5955 1 36] BP_Implementable
  (Utilities|IsValid Causer
    (:Is%20Valid
      (if (Actor|ActorHasTag Causer "Player")
        (bind _asmain_character_base (Utilities|Casting|CastToMainCharacterBase Causer)
          (:then
            (Utilities|FlowControl|DoOnce false :!label _label
              (:Completed
                (bind _returnvalue (Class|CharacterBase|PickWeapon _asmain_character_base (Math|Conversions|ToInteger(Byte) (Variables|Default|GetItemID))))
                (if _returnvalue
                  (Actor|DestroyActor)
                  (else
                    (goto _label Reset))))))
          (:CastFailed
            (Development|PrintString "Cast Failed")))
        (else
          (Development|PrintString "NO tag"))))
    (:Is%20Not%20Valid
      (Development|PrintString "InValid  Player"))))

(fn ConstructionScript)