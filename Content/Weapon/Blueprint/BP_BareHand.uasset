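; BP_BareHand is a weapon Blueprint, apparently the unarmed option, with a Sphere component and a WeaponMesh.
; On Sphere overlap it checks validity, the Player tag and a cast to MainCharacterBase, but takes no action afterwards.
; A disconnected chain that would destroy the Sphere after a short delay and set the weapon mesh never runs, and the construction script is empty.
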(event OnComponentBeginOverlap(Sphere)
  (params (OverlappedComponent :type Primitive%20Component%20Object%20Reference) (OtherActor :type Actor%20Object%20Reference) (OtherComp :type Primitive%20Component%20Object%20Reference) (OtherBodyIndex :type Integer) (bFromSweep :type Boolean) (SweepResult :type Hit%20Result%20Structure%20%28by%20ref%29))
  (Utilities|IsValid (Variables|Default|GetSphere)
    (:Is%20Valid
      (Utilities|IsValid OtherActor
        (:Is%20Valid
          (if (and (Actor|ActorHasTag OtherActor "Player") (.bSuccess (Utilities|Casting|CastToMainCharacterBase OtherActor)))
            _))))))

(fn ConstructionScript)