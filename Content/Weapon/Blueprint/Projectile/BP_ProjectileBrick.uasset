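; BP_ProjectileBrick is a brick weapon projectile whose movement is tuned from a ProjectileStat struct.
; The construction script copies speed into the movement component's initial and maximum speed and also sets its gravity scale.
; The event graph holds disconnected, never-executed logic that would turn on homing toward a Character-tagged actor other than the owner.
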(fn ConstructionScript
  (bind _projectilemovement (Variables|Default|GetProjectileMovement))
  (bind _projectilestat (Variables|Default|GetProjectileStat))
  (bind (_projectilename _description _bisexplosive _projectilespeed _projectiledamage _gravityscale) (Utilities|Struct|BreakProjectileStatStruct _projectilestat))
  (Variables|/Script/Engine.ProjectileMovementComponent|SetInitialSpeed _projectilemovement _projectilespeed)
  (Variables|/Script/Engine.ProjectileMovementComponent|SetMaxSpeed _projectilemovement _projectilespeed)
  (Variables|/Script/Engine.ProjectileMovementComponent|SetProjectileGravityScale _projectilemovement _gravityscale))