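; BP_GlassBottle is a glass bottle weapon that characters pick up by walking into it.
; Its Sphere overlap only responds while the bottle has no owner, accepting actors tagged Character that cast to CharacterBase.
; On a valid overlap it disables the Sphere's collision, scales it to zero and passes itself to the character's PickWeapon.
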(event OnComponentBeginOverlap(Sphere)
  (params (OverlappedComponent :type Primitive%20Component%20Object%20Reference) (OtherActor :type Actor%20Object%20Reference) (OtherComp :type Primitive%20Component%20Object%20Reference) (OtherBodyIndex :type Integer) (bFromSweep :type Boolean) (SweepResult :type Hit%20Result%20Structure%20%28by%20ref%29))
  (bind (_ascharacter_base _bsuccess) (Utilities|Casting|CastToCharacterBase OtherActor))
  (bind _sphere (Variables|Default|GetSphere))
  (Utilities|IsValid (Components|GetOwner)
    (:Is%20Not%20Valid
      (Utilities|IsValid (Variables|Default|GetSphere)
        (:Is%20Valid
          (if (Math|Boolean|ANDBoolean (Utilities|IsValid OtherActor) (Actor|ActorHasTag OtherActor "Character") _bsuccess)
            (Collision|SetCollisionEnabled _sphere "NoCollision")
            (Transformation|SetWorldScale3D _sphere "0, 0, 0")
            (Class|CharacterBase|PickWeapon _ascharacter_base self)))))))

(fn ConstructionScript)