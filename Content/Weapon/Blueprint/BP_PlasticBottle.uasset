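; Plastic bottle weapon that a character picks up by walking into its Sphere trigger.
; On overlap, it requires an actor tagged "Character" that casts to CharacterBase, then passes itself to that character's InitWeapon.
; It then destroys the Sphere component, so the pickup fires only once while the bottle actor itself remains.
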(event OnComponentBeginOverlap(Sphere)
  (params (OverlappedComponent :type Primitive%20Component%20Object%20Reference) (OtherActor :type Actor%20Object%20Reference) (OtherComp :type Primitive%20Component%20Object%20Reference) (OtherBodyIndex :type Integer) (bFromSweep :type Boolean) (SweepResult :type Hit%20Result%20Structure%20%28by%20ref%29))
  (bind (_ascharacter_base _bsuccess) (Utilities|Casting|CastToCharacterBase OtherActor))
  (Utilities|IsValid (Variables|Default|GetSphere)
    (:Is%20Valid
      (if (Math|Boolean|ANDBoolean (Utilities|IsValid OtherActor) (Actor|ActorHasTag OtherActor "Character") _bsuccess)
        (Class|CharacterBase|InitWeapon _ascharacter_base self)
        (Components|DestroyComponent (Variables|Default|GetSphere))))))

(fn ConstructionScript)