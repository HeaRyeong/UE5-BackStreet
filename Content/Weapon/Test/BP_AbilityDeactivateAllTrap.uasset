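; Test trap actor that strips all character abilities from a player who walks into its box.
; On overlap, actors tagged both Character and Player are cast to MainCharacterBase, and a loop over every ECharacterAbilityType calls TryRemoveAbility.
; Each removal result is printed on screen for debugging.
; A DoOnce gate blocks retriggering until a short delay after the loop finishes resets it.
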(event OnComponentBeginOverlap(Box)
  (params (OverlappedComponent :type Primitive%20Component%20Object%20Reference) (OtherActor :type Actor%20Object%20Reference) (OtherComp :type Primitive%20Component%20Object%20Reference) (OtherBodyIndex :type Integer) (bFromSweep :type Boolean) (SweepResult :type Hit%20Result%20Structure%20%28by%20ref%29))
  (Utilities|IsValid OtherActor
    (:Is%20Valid
      (if (Actor|ActorHasTag OtherActor "Character")
        (if (Actor|ActorHasTag OtherActor "Player")
          (Utilities|FlowControl|DoOnce false :!label _label
            (:Completed
              (bind _asmain_character_base (Utilities|Casting|CastToMainCharacterBase OtherActor))
              (bind _enumvalue (|ForEachECharacterAbilityType)
                (:LoopBody
                  (bind _returnvalue (Class|MainCharacterBase|TryRemoveAbility _asmain_character_base _enumvalue))
                  (Development|PrintString (Utilities|String|Append (Utilities|String|ToString(Byte) _enumvalue) " : " (Utilities|String|ToString(Boolean) _returnvalue)) true false "(R=1.000000,G=0.415821,B=0.156726,A=1.000000)"))
                (:then
                  (Utilities|FlowControl|Delay 5.0)
                  (goto _label Reset))))))))))

(event EventBeginPlay)

(event Collision|EventActorBeginOverlap
  (params (OtherActor :type Actor%20Object%20Reference)))

(event EventTick
  (params (DeltaSeconds :type Float%20%28single-precision%29)))

(fn ConstructionScript)