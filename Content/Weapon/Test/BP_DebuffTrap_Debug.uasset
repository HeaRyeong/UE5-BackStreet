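; Debug trap actor that applies a configurable debuff to characters entering its Box trigger.
; Overlapping actors tagged Character are split by the Player tag into MainCharacterBase or EnemyCharacterBase casts, then receive AddNewBuffDebuff with the trap's type, duration and value.
; Each branch has its own DoOnce reset after a five-second delay, so the cooldown is shared by all enemies rather than tracked per actor.
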(event OnComponentBeginOverlap(Box)
  (params (OverlappedComponent :type Primitive%20Component%20Object%20Reference) (OtherActor :type Actor%20Object%20Reference) (OtherComp :type Primitive%20Component%20Object%20Reference) (OtherBodyIndex :type Integer) (bFromSweep :type Boolean) (SweepResult :type Hit%20Result%20Structure%20%28by%20ref%29))
  (bind _self self)
  (bind _debuff_type (Variables|Default|GetDebuff%20Type))
  (bind _total_time (Variables|Default|GetTotal%20Time))
  (bind _variable (Variables|Default|GetVariable))
  (Utilities|IsValid OtherActor
    (:Is%20Valid
      (if (Actor|ActorHasTag OtherActor "Character")
        (if (Actor|ActorHasTag OtherActor "Player")
          (Utilities|FlowControl|DoOnce false :!label _label
            (:Completed
              (bind _asmain_character_base (Utilities|Casting|CastToMainCharacterBase OtherActor))
              (Class|MainCharacterBase|AddNewBuffDebuff _asmain_character_base true _debuff_type _self _total_time _variable)
              (Utilities|FlowControl|Delay 5.0)
              (goto _label Reset)))
          (else
            (Utilities|FlowControl|DoOnce false :!label _label_2
              (:Completed
                (bind _asenemy_character_base (Utilities|Casting|CastToEnemyCharacterBase OtherActor))
                (Class|EnemyCharacterBase|AddNewBuffDebuff _asenemy_character_base true _debuff_type _self _total_time _variable)
                (Utilities|FlowControl|Delay 5.0)
                (goto _label_2 Reset)))))))))

(event EventBeginPlay)

(event Collision|EventActorBeginOverlap
  (params (OtherActor :type Actor%20Object%20Reference)))

(event EventTick
  (params (DeltaSeconds :type Float%20%28single-precision%29)))

(fn ConstructionScript)