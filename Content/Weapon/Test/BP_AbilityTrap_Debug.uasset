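; BP_AbilityTrap_Debug is a debug trigger that toggles an ability on the player for testing.
; When an actor tagged both Character and Player overlaps its Box, it casts to MainCharacterBase and asks the ability manager whether AbilityType is active.
; It removes an active ability or adds an inactive one, then prints the result.
; A DoOnce that resets after a short delay throttles repeated toggles.
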(event OnComponentBeginOverlap(Box)
  (params (OverlappedComponent :type Primitive%20Component%20Object%20Reference) (OtherActor :type Actor%20Object%20Reference) (OtherComp :type Primitive%20Component%20Object%20Reference) (OtherBodyIndex :type Integer) (bFromSweep :type Boolean) (SweepResult :type Hit%20Result%20Structure%20%28by%20ref%29))
  (bind _ability_type (Variables|Default|GetAbility%20Type))
  (Utilities|IsValid OtherActor
    (:Is%20Valid
      (if (Actor|ActorHasTag OtherActor "Character")
        (if (Actor|ActorHasTag OtherActor "Player")
          (Utilities|FlowControl|DoOnce false :!label _label
            (:Completed
              (bind _asmain_character_base (Utilities|Casting|CastToMainCharacterBase OtherActor))
              (if (Class|AbilityManagerBase|GetIsAbilityActive (Class|MainCharacterBase|GetAbilityManagerRef _asmain_character_base) (Variables|Default|GetAbility%20Type))
                (bind _returnvalue (Class|MainCharacterBase|TryRemoveAbility _asmain_character_base _ability_type))
                (Development|PrintString (Utilities|String|ToString(Boolean) _returnvalue))
                (else
                  (bind _returnvalue_2 (Class|MainCharacterBase|TryAddNewAbility _asmain_character_base _ability_type))
                  (Development|PrintString (Utilities|String|ToString(Boolean) _returnvalue_2))))
              (Utilities|FlowControl|Delay 2.0)
              (goto _label Reset))))))))

(event EventBeginPlay)

(event Collision|EventActorBeginOverlap
  (params (OtherActor :type Actor%20Object%20Reference)))

(event EventTick
  (params (DeltaSeconds :type Float%20%28single-precision%29)))

(fn ConstructionScript)