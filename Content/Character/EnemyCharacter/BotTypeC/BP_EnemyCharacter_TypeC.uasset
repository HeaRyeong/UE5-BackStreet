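; BP_EnemyCharacter_TypeC is the Blueprint for the Type C enemy character, adding HP bar setup and damage debugging.
; InitFloatingHpWidget, an implementable event, casts the FloatingHpBar component's widget to WB_EnemyHPBar and sets this enemy as its owner.
; A debug AnyDamage handler waits briefly, then prints the damage and the current HP from CharacterState in yellow.
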(event EventInitFloatingHpWidget
  (bind _floatinghpbar (Variables|Default|GetFloatingHpBar))
  (bind _returnvalue (UserInterface|GetWidget _floatinghpbar))
  ;[1 1 1] BP_ImplementableEvent
  (Utilities|IsValid _returnvalue
    (:Is%20Valid
      (bind _aswb_enemy_hpbar (Utilities|Casting|CastToWB_EnemyHPBar _returnvalue))
      (Default|SetOwnerRef _aswb_enemy_hpbar self))))

(event Game|Damage|EventAnyDamage
  (params (Damage :type Float%20%28single-precision%29) (DamageType :type Damage%20Type%20Object%20Reference) (InstigatedBy :type Controller%20Object%20Reference) (DamageCauser :type Actor%20Object%20Reference))
  ;[1 1 1] Debug
  (Utilities|FlowControl|Delay 0.2)
  (Development|PrintString (Utilities|String|Append "Damage : " (Utilities|String|ToString(Float) Damage) " / CurrHP : " (Utilities|String|ToString(Float) (.CharacterCurrHP (Utilities|Struct|BreakCharacterStateStruct (Variables|Default|GetCharacterState))))) true true "(R=1.000000,G=0.916800,B=0.000000,A=1.000000)"))

(fn ConstructionScript)