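; Main character Blueprint that adds per-frame debug readouts and camera occlusion feedback to the player.
; Tick prints buff and debuff flags, action state, stats, HP, ammo and inventory weapon info on screen.
; CheckWall line-traces forward from the following camera, swapping the mesh to a "Visible" material when the hit actor lacks the Player tag.
; An IsBlock flag limits material swaps to state changes; CheckWall is marked for moving to native code.
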(event Custom|CheckWall
  (bind _followingcamera (Variables|Default|GetFollowingCamera))
  (bind _returnvalue (Transformation|GetWorldLocation _followingcamera))
  ;[1 1 1] 네이티브화 필요
  (bind (_outhit _returnvalue_2) (Collision|LineTraceByChannel _returnvalue (+ _returnvalue (* (Math|Vector|GetForwardVector (Transformation|GetWorldRotation _followingcamera)) 5e+03)) "TraceTypeQuery2" false 0 "None" false))
  (if _returnvalue_2
    (if (Actor|ActorHasTag (.HitActor (Collision|BreakHitResult _outhit)) "Player")
      (if (Variables|Default|GetIsBlock)
        (Rendering|Material|SetMaterial (Variables|Character|GetMesh) 0 "/Game/Asset/Characters/Cute_cardboard_boy/Material/Mat_Cute_cardboard_boy.Mat_Cute_cardboard_boy")
        (Variables|Default|SetIsBlock false))
      (elif (not (Variables|Default|GetIsBlock))
        (Rendering|Material|SetMaterial (Variables|Character|GetMesh) 0 "/Game/Character/MainCharacter/Material/Mat_Cute_cardboard_boy_Visible.Mat_Cute_cardboard_boy_Visible")
        (Variables|Default|SetIsBlock true)))))

(event EventTick
  (params (DeltaSeconds :type Float%20%28single-precision%29))
  (bind _returnvalue (Class|CharacterBase|GetWeaponActorRef))
  ;[0.9571 0 1 1 50] Tick / Debug
  (CallFunction|PrintCharacterInfo)
  (CallFunction|CheckWall)
  (bind _returnvalue_2 (Class|CharacterBase|GetInventoryRef))
  (Utilities|IsValid _returnvalue_2
    (:Is%20Valid
      (Utilities|IsValid _returnvalue
        (:Is%20Valid
          (Development|PrintString (Utilities|String|Append "Inventory Idx : " (Utilities|String|ToString(Integer) (Class|WeaponInventoryBase|GetCurrentIdx _returnvalue_2)) "   /   " "Weapon Count  :  " (Utilities|String|ToString(Integer) (Class|WeaponInventoryBase|GetCurrentWeaponCount _returnvalue_2)) "  /  Weapon Name : " (Utilities|String|SelectString (Utilities|String|ToString(Name) (.WeaponName (Utilities|Struct|BreakWeaponStatStruct (Variables|/Script/BackStreet.WeaponBase|GetWeaponStat _returnvalue)))) "None" (Utilities|IsValid _returnvalue))) true false "(R=0.000000,G=0.660000,B=1.000000,A=1.000000)" 0.01))))))

(event Input|ActionEvents|InputActionWeaponSwitch
  (params (Key :type Key%20Structure :default "None"))
  ;[1 0.4045 0.3047 1 50] Work In Progress
)

(fn ConstructionScript)

(fn PrintCharacterInfo
  (bind _returnvalue (Class|CharacterBase|GetWeaponActorRef))
  (bind _characterstate (Variables|Default|GetCharacterState))
  (bind _characterstat (Variables|Default|GetCharacterStat))
  (bind (_characterdebuffstate _characterbuffstate _bcanattack _turndirection _characteractionstate _charactercurrhp) (Utilities|Struct|BreakCharacterStateStruct _characterstate))
  (bind (_bisinvincibility _binfiniteammo _binfinitedurability _charactermaxhp _characteratkmultiplier _characteratkspeed _charactermovespeed _characterdefense) (Utilities|Struct|BreakCharacterStatStruct _characterstat))
  (bind _weaponstate (Variables|/Script/BackStreet.WeaponBase|GetWeaponState _returnvalue))
  (bind (_currentdurability _combocount _currentammocount _totalammocount) (Utilities|Struct|BreakWeaponStateStruct _weaponstate))
  (Utilities|FlowControl|Sequence
    (:then_0
      (for _index (range 0 8)
        (LocalVariables|SetTemp (Utilities|String|Append (LocalVariables|GetTemp) (Utilities|String|Append (Utilities|String|EnumtoString (Utilities|Enum|ByteToEnumECharacterDebuffType (Math|Conversions|ToByte(Integer) _index))) " : " (Utilities|String|ToString(Boolean) (Class|CharacterBase|GetDebuffIsActive (Utilities|Enum|ByteToEnumECharacterDebuffType (Math|Conversions|ToByte(Integer) _index)))) " / "))))
      (Development|PrintString (LocalVariables|GetTemp) true false "(R=0.480775,G=1.000000,B=0.463542,A=1.000000)" 0.003)
      (LocalVariables|SetTemp ""))
    (:then_1
      (for _index_2 (range 0 8)
        (LocalVariables|SetTemp (Utilities|String|Append (LocalVariables|GetTemp) (Utilities|String|Append (Utilities|String|EnumtoString (Utilities|Enum|ByteToEnumECharacterBuffType (Math|Conversions|ToByte(Integer) _index_2))) " : " (Utilities|String|ToString(Boolean) (Class|CharacterBase|GetBuffIsActive (Utilities|Enum|ByteToEnumECharacterBuffType (Math|Conversions|ToByte(Integer) _index_2)))) " / "))))
      (Development|PrintString (LocalVariables|GetTemp) true false "(R=0.480775,G=1.000000,B=0.463542,A=1.000000)" 0.003)
      (LocalVariables|SetTemp ""))
    (:then_2
      (Development|PrintString (Utilities|String|Append "ActionState :  " (Utilities|String|EnumtoString _characteractionstate) "  /  Can Atk : " (Utilities|String|ToString(Boolean) _bcanattack)) true false "(R=1.000000,G=0.955652,B=0.000000,A=1.000000)" 0.003))
    (:then_3
      (Development|PrintString (Utilities|String|Append "Speed : " (Utilities|String|ToString(Float) (Variables|/Script/Engine.CharacterMovementComponent|GetMaxWalkSpeed (Variables|Character|GetCharacterMovement))) ", " (Utilities|String|ToString(Float) _charactermovespeed) "  /  Atk Speed : " (Utilities|String|ToString(Float) _characteratkspeed)) true false "(R=0.000000,G=0.900125,B=1.000000,A=1.000000)" 0.003))
    (:then_4
      (Development|PrintString (Utilities|String|Append "DEF : " (Utilities|String|ToString(Float) _characterdefense) "/ ATK : " (Utilities|String|ToString(Float) _characteratkmultiplier)) true false "(R=0.000000,G=0.363636,B=1.000000,A=1.000000)" 0.003))
    (:then_5
      (Development|PrintString (Utilities|String|Append "HP : " (Utilities|String|ToString(Float) _charactercurrhp) "/" (Utilities|String|ToString(Float) _charactermaxhp)) true false "(R=1.000000,G=0.227609,B=0.223958,A=1.000000)" 0.003))
    (:then_6
      (Utilities|IsValid _returnvalue
        (:Is%20Valid
          (if (and (Utilities|IsValid _returnvalue) (.bHasProjectile (Utilities|Struct|BreakWeaponStatStruct (Variables|/Script/BackStreet.WeaponBase|GetWeaponStat _returnvalue))))
            (Development|PrintString (Utilities|String|Append "Ammo : " (Utilities|String|ToString(Integer) _currentammocount) "/" (Utilities|String|ToString(Integer) _totalammocount)) true false "(R=1.000000,G=0.647500,B=0.645833,A=1.000000)" 0.003)))))))