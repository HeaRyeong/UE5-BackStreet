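; BP_ChapterGate is a gate actor that advances the game to the next chapter, and it destroys itself on BeginPlay unless the current tile is a boss stage.
; When the player overlaps it and the chapter's mission stage array is empty, it checks the game mode's remaining chapter count.
; It either prints Game Clear or initializes a new chapter, loads the current tile's level and teleports the player above that tile.
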(event EventBeginPlay
  (bind _asbp_back_street_game_mode (Utilities|Casting|CastToBP_BackStreetGameMode (Game|GetGameMode)))
  (if (not (Variables|/Script/BackStreet.TileBase|GetbIsBossStage (Variables|/Script/BackStreet.BackStreetGameModeBase|GetCurrTile _asbp_back_street_game_mode)))
    (Actor|DestroyActor)))

(event Collision|EventActorBeginOverlap
  (params (OtherActor :type Actor%20Object%20Reference))
  (if (Actor|ActorHasTag OtherActor "Player")
    (bind _asbp_back_street_game_mode (Utilities|Casting|CastToBP_BackStreetGameMode (Game|GetGameMode)))
    (if (Utilities|Array|IsEmpty (Variables|/Script/BackStreet.GridBase|GetMissionStageArray (Variables|/Script/BackStreet.BackStreetGameModeBase|GetChapter _asbp_back_street_game_mode)))
      (if (== (Variables|/Script/BackStreet.BackStreetGameModeBase|GetRemainChapter _asbp_back_street_game_mode) 0)
        (Development|PrintString "Game Clear")
        (else
          (Development|PrintString "Chapter Clear")
          (Class|BackStreetGameModeBase|InitChapter _asbp_back_street_game_mode)
          (Class|TileBase|LoadLevel (Variables|/Script/BackStreet.BackStreetGameModeBase|GetCurrTile _asbp_back_street_game_mode))
          (Transformation|SetActorLocation (Game|GetPlayerCharacter 0) (Math|Vector|MakeVector (.x (Transformation|GetActorLocation (Variables|/Script/BackStreet.BackStreetGameModeBase|GetCurrTile _asbp_back_street_game_mode))) (.y (Transformation|GetActorLocation (Variables|/Script/BackStreet.BackStreetGameModeBase|GetCurrTile _asbp_back_street_game_mode))) 5e+02) false false))))))

(event EventTick
  (params (DeltaSeconds :type Float%20%28single-precision%29)))

(fn ConstructionScript)