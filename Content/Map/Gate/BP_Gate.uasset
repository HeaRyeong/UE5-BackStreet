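; BP_Gate is a stage exit gate that moves the player on to another level once the current tile is cleared.
; On overlap with an actor tagged Player, it checks the current tile's clear flag on BP_BackStreetGameMode.
; If clear, it updates its gate info, has the game mode load a level and unload using that info, then destroys itself.
; Otherwise it prints a prompt to clear the stage.
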(event EventBeginPlay)

(event Collision|EventActorBeginOverlap
  (params (OtherActor :type Actor%20Object%20Reference))
  (if (Actor|ActorHasTag OtherActor "Player")
    (bind _asbp_back_street_game_mode (Utilities|Casting|CastToBP_BackStreetGameMode (Game|GetGameMode)))
    (if (Variables|/Script/BackStreet.Tile|GetIsClear (Variables|/Script/BackStreet.BackStreetGameModeBase|GetCurrTile _asbp_back_street_game_mode))
      (Development|PrintText "Stage Clear")
      (bind _returnvalue (Class|Gate|UpdateGateInfo))
      (Default|LoadLevel _asbp_back_street_game_mode)
      (Default|UnLoadLevel _asbp_back_street_game_mode _returnvalue)
      (Actor|DestroyActor)
      (else
        (Development|PrintText "Please Clear Stage")))))

(event EventTick
  (params (DeltaSeconds :type Float%20%28single-precision%29)))

(fn ConstructionScript)