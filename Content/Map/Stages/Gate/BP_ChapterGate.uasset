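; Chapter exit gate that exists only on boss stages and moves the player on to the next chapter.
; On BeginPlay it reads the current tile from BackStreetGameModeBase and destroys itself if that tile is not a boss stage.
; When the player overlaps it with no mission stages left, it either prints a game-clear message or initializes the next chapter, loads the current tile's level and teleports the player above it.
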(event EventBeginPlay
  (bind _asback_street_game_mode_base (Utilities|Casting|CastToBackStreetGameModeBase (Game|GetGameMode)))
  (if (not (Variables|/Script/BackStreet.Tile|GetbIsBossStage (Variables|/Script/BackStreet.BackStreetGameModeBase|GetCurrTile _asback_street_game_mode_base)))
    (Actor|DestroyActor)))

(event Collision|EventActorBeginOverlap
  (params (OtherActor :type Actor%20Object%20Reference))
  (if (Actor|ActorHasTag OtherActor "Player")
    (bind _asback_street_game_mode_base (Utilities|Casting|CastToBackStreetGameModeBase (Game|GetGameMode)))
    (if (Utilities|Array|IsEmpty (Variables|/Script/BackStreet.Grid|GetMissionStageArray (Variables|/Script/BackStreet.BackStreetGameModeBase|GetChapter _asback_street_game_mode_base)))
      (if (== (Variables|/Script/BackStreet.BackStreetGameModeBase|GetRemainChapter _asback_street_game_mode_base) 0)
        (Development|PrintString "Game Clear")
        (else
          (Development|PrintString "Chapter Clear")
          (Class|BackStreetGameModeBase|InitChapter _asback_street_game_mode_base)
          (Class|Tile|LoadLevel (Variables|/Script/BackStreet.BackStreetGameModeBase|GetCurrTile _asback_street_game_mode_base))
          (Transformation|SetActorLocation (Game|GetPlayerCharacter 0) (Math|Vector|MakeVector (.x (Transformation|GetActorLocation (Variables|/Script/BackStreet.BackStreetGameModeBase|GetCurrTile _asback_street_game_mode_base))) (.y (Transformation|GetActorLocation (Variables|/Script/BackStreet.BackStreetGameModeBase|GetCurrTile _asback_street_game_mode_base))) 5e+02) false false))))))

(event EventTick
  (params (DeltaSeconds :type Float%20%28single-precision%29)))

(fn ConstructionScript)