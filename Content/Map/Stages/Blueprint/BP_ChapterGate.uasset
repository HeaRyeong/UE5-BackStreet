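; BP_ChapterGate is a map gate actor that lets the player finish a chapter from a boss stage.
; On BeginPlay it destroys itself unless the game mode's current tile is a boss stage.
; When an actor tagged Player overlaps it, it calls ClearChapter on the game mode if the chapter is flagged clear, otherwise it prints a message to clear missions.
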(event EventBeginPlay
  (bind _asbp_back_street_game_mode (Utilities|Casting|CastToBP_BackStreetGameMode (Game|GetGameMode)))
  (if (not (Variables|/Script/BackStreet.TileBase|GetbIsBossStage (Variables|/Script/BackStreet.BackStreetGameModeBase|GetCurrTile _asbp_back_street_game_mode)))
    (Actor|DestroyActor)))

(event Collision|EventActorBeginOverlap
  (params (OtherActor :type Actor%20Object%20Reference))
  (if (Actor|ActorHasTag OtherActor "Player")
    (bind _asbp_back_street_game_mode (Utilities|Casting|CastToBP_BackStreetGameMode (Game|GetGameMode)))
    (if (Variables|/Script/BackStreet.GridBase|GetbIsChapterClear (Variables|/Script/BackStreet.BackStreetGameModeBase|GetChapter _asbp_back_street_game_mode))
      (Class|BackStreetGameModeBase|ClearChapter _asbp_back_street_game_mode)
      (else
        (Development|PrintString "Please  Clear Missoins")))))

(event EventTick
  (params (DeltaSeconds :type Float%20%28single-precision%29)))

(fn ConstructionScript)