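; BP_RewardBox is a reward box actor that offers an ability, identified by PossessAbilityID, to the player.
; Player overlap shows a widget component popup with the ability's icon from AbilityImageMap and hides it when the player leaves.
; EnterUI refreshes the character's ability list and opens WB_SelectReward in UI-only input, passing it the box's ability and the character's A and B abilities.
; UpdateUI refreshes that screen's images.
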(event EventUpdateUI
  (Default|SetUIImage (stale EventEnterUI _returnvalue) (Variables|Default|GetPossessAbilityID) (Variables|Default|GetCharacterAbilityIDA) (Variables|Default|GetCharacterAbilityIDB)))

(event EventEnterUI
  (bind _possessabilityid (Variables|Default|GetPossessAbilityID))
  (Class|RewardBox|SetCharacterAbilityList)
  (bind _returnvalue (Game|ConstructObjectfromClass "/Game/UI/InGame/Blueprint/Component/WB_SelectReward.WB_SelectReward_C" _possessabilityid))
  (UserInterface|Viewport|AddtoViewport _returnvalue 0)
  (Input|SetInputModeUIOnly (Game|GetPlayerController 0) _returnvalue "DoNotLock")
  (Default|InitUIVar _returnvalue (Variables|Default|GetAbilityImageMap))
  (Default|SetUIImage _returnvalue _possessabilityid (Variables|Default|GetCharacterAbilityIDA) (Variables|Default|GetCharacterAbilityIDB)))

(event EventTick
  (params (DeltaSeconds :type Float%20%28single-precision%29)))

(event Collision|EventActorEndOverlap
  (params (OtherActor :type Actor%20Object%20Reference))
  (if (== OtherActor (Game|GetPlayerCharacter 0))
    (Rendering|SetVisibility (Variables|Default|GetWidget) false false)))

(event Collision|EventActorBeginOverlap
  (params (OtherActor :type Actor%20Object%20Reference))
  (bind _widget (Variables|Default|GetWidget))
  (if (== OtherActor (Game|GetPlayerCharacter 0))
    (Utilities|IsValid _widget
      (:Is%20Valid
        (bind _aswb_reward_box_pop_up (Utilities|Casting|CastToWB_RewardBoxPopUp (UserInterface|GetWidget (Variables|Default|GetWidget))))
        (Default|SetAbilityImage _aswb_reward_box_pop_up (Variables|Default|GetPossessAbilityID) (Variables|Default|GetAbilityImageMap))
        (Rendering|SetVisibility _widget true false))
      (:Is%20Not%20Valid
        (Development|PrintString "Hello")))))

(fn ConstructionScript)